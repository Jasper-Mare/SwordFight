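; Pavlov custom game mode for a two-team sword fight, with auto respawn and custom kill scoring.
; Round state changes drive the match: wait for players (minimum one), scatter chickens during stand-by, spawn pawns and run the respawn loop, then end the match.
; Kills by others score for killer and team, while dying costs a point.
; Each spawn grants a random, enlarged team weapon and sets the team skin.
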(event EventBeginPlay
  (|CallParentFunction))

(event EventTick
  (params (DeltaSeconds :type Float%20%28single-precision%29))
  (|CallParentFunction DeltaSeconds))

(event EventOnRoundStateChanged
  (params (OldState :type EPavlovRoundState%20Enum :default "Starting") (NewState :type EPavlovRoundState%20Enum :default "Starting"))
  (switch Utilities|FlowControl|Switch|SwitchonEPavlovRoundState NewState
    (:Starting
      (Utilities|FlowControl|Delay 1.0)
      (CallFunction|StartWaitforPlayersLoop))
    (:StandBy
      (Utilities|FlowControl|Delay 1.0)
      (for _index (range 1 10)
        (Class|PavlovGameLogic|SpawnChicken (Math|Transform|MakeTransform (Math|Vector|MakeVector (Math|Random|RandomFloatinRange -1e+03 1e+03) (Math|Random|RandomFloatinRange -1e+03 1e+03) 2e+01))))
      (Utilities|FlowControl|Delay 3.0)
      (Class|PavlovGameLogic|SetRoundState "Started"))
    (:Started
      (Utilities|FlowControl|Delay 1.0)
      (Class|PavlovGameLogic|SpawnandPosessPawns)
      (CallFunction|StartRespawnLoop))
    (:Ended
      (CallFunction|StopRespawnLoop)
      (Utilities|FlowControl|Delay 5.0)
      ;[1 1 1] To go back to lobby/rotate to next map
      (bind _asgame_mode (Utilities|Casting|CastToGameMode (Game|GetGameMode)))
      (Class|GameMode|EndMatch _asgame_mode))))

(event EventOnCustomGameModeInit
  (Class|PavlovGameLogic|SetGameModeProperties (Utilities|Struct|MakePavlovGameModeProperties false false true 0 0 0 false true 5.0 false false 60 10 true true 900)))

(event EventOnPlayerKilled
  (params (PlayerStatus :type Pavlov%20Player%20Status%20Structure%20%28by%20ref%29) (Killer :type Player%20State%20Object%20Reference) (bHeadshot :type Boolean) (KilledByItem :type Name :default "None"))
  (bind (_playerstate _controller _pawn _steamid _cash _score) (Utilities|Struct|BreakPavlovPlayerStatus PlayerStatus))
  (if (!= Killer _playerstate)
    (Class|PavlovGameLogic|IncrementPlayerScore Killer 2)
    (bind _returnvalue (Class|PavlovPlayerInfo|GetTeam (Class|PavlovLibrary|GetPlayerInfo Killer)))
    (Class|PavlovGameLogic|IncrementTeamScore _returnvalue 1))
  (if (> _score 0)
    (Class|PavlovGameLogic|IncrementPlayerScore _playerstate -1)))

(fn ConstructionScript
  (|CallParentFunction))

(fn PlayerSpawned
  (params (PlayerStatus :type Pavlov%20Player%20Status%20Structure%20%28by%20ref%29))
  (bind (_playerstate _controller _pawn _steamid _cash _score _teamid _health _armour _bhelmet _bdead _bcanbuy _bcrouching _bgagged _brighthanded) (Utilities|Struct|BreakPavlovPlayerStatus PlayerStatus))
  (bind _spawnweaponsteam1 (Variables|Default|GetSpawnWeaponsTeam1))
  (bind _spawnweaponsteam2 (Variables|Default|GetSpawnWeaponsTeam2))
  (bind _returnvalue (Utilities|Select :Index _teamid :Option%200 _spawnweaponsteam1 :Option%201 _spawnweaponsteam2))
  (bind (_bsuccessful _item) (Class|PavlovGameLogic|SpawnItemWRef (Class|PavlovLibrary|GetGameLogic) (Utilities|Struct|MakePavlovItemSpawnParams :Id (Utilities|Array|Get(acopy) _returnvalue (Math|Random|RandomInteger (Utilities|Array|Length _returnvalue))) :Player _playerstate :bDominantHand false :bSpawnInInventory true :InventorySlot (Math|Conversions|ToInteger(Boolean) _brighthanded) :bSpawnWithDefaultAttachments false)))
  (Transformation|SetActorScale3D _item "1.500000,1.500000,3.000000")
  (Class|PavlovPlayerInfo|SetRadioChannel (Class|PavlovLibrary|GetPlayerInfo _playerstate))
  (Class|PavlovPlayerProxy|SetPlayerSkin (Class|PavlovLibrary|GetPlayerProxy _pawn) (Utilities|Select :Index _teamid :Option%200 "russian" :Option%201 "us"))
  (return _bsuccessful))

(fn EnoughPlayerstoStart
  (params (PlayerCountToStart :type Integer))
  (bind _hasenough (|CallParentFunction 1))
  (return _hasenough))