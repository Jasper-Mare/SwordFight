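; Custom player Blueprint for the Jasper SwordFight custom map that enlarges whatever the player holds.
; Every Tick it queries GetHeldItem for both values of its boolean flag, presumably one per hand, and sets each found item's actor scale, stretching it most along Z.
; No item type filter applies, as an unconnected "bayonet" name-prefix check never runs.
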(event EventBeginPlay)

(event EventTick
  (params (DeltaSeconds :type Float%20%28single-precision%29))
  (Utilities|FlowControl|Sequence
    (:then_0
      (bind (_bhasitem _item) (Class|PavlovPlayerProxy|GetHeldItem false))
      (if _bhasitem
        (Transformation|SetActorScale3D (.Item (Utilities|Struct|BreakPlayerItem _item)) "1.500000,1.500000,3.000000")))
    (:then_1
      (bind (_bhasitem_2 _item_2) (Class|PavlovPlayerProxy|GetHeldItem true))
      (if _bhasitem_2
        (Transformation|SetActorScale3D (.Item (Utilities|Struct|BreakPlayerItem _item_2)) "1.500000,1.500000,3.000000")))))

(event Collision|EventActorBeginOverlap
  (params (OtherActor :type Actor%20Object%20Reference)))

(fn ConstructionScript)